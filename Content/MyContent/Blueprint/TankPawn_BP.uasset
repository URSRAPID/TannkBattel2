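; Player-controllable tank pawn Blueprint that wires input to camera, movement and firing.
; On BeginPlay it hands the cannon and turret to a TankAiming component and both tracks to a TankMovement component.
; Azimuth and elevation axes rotate a gimbal and spring arm separately, scaled by delta time, for camera orbit.
; Move and turn axes pass intent to TankMovement, and the Fire action calls Fire.
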(event EventBeginPlay
  (Class|TankAimingComponent|InitializeAIM (Variables|Default|GetTankAiming) (Variables|Default|GetCanon1) (Variables|Default|GetTurret))
  (Class|TankMovementComponent|Initialize (Variables|Default|GetTankMovement) (Variables|Default|GetLeftTrack) (Variables|Default|GetRightTrack)))

(event Collision|EventActorBeginOverlap
  (params (OtherActor :type Actor%20Object%20Reference)))

(event EventTick
  (params (DeltaSeconds :type Float%20%28single-precision%29)))

(event Input|ActionEvents|InputActionFire
  (params (Key :type Key%20Structure))
  ;[1 0.3467 0.1661] Fire Input
  (:Pressed
    (Class|Tank|Fire)))

(event Input|AxisEvents|InputAxisRotateAzimuth
  (params (AxisValue :type Float%20%28single-precision%29))
  ;[0.1517 0.6511 1] Camera Rotation
  (Transformation|AddLocalRotation (Variables|Default|GetAzimuthGimbal) (Math|Rotator|MakeRotator 0.0 0.0 (* AxisValue (Utilities|Time|GetWorldDeltaSeconds) 1e+02)) false false))

(event Input|AxisEvents|InputAxisRotateElevation
  (params (AxisValue :type Float%20%28single-precision%29))
  ;[0.1517 0.6511 1] Camera Rotation
  (Transformation|AddLocalRotation (Variables|Default|GetSpringArm) (Math|Rotator|MakeRotator 0.0 (* AxisValue (Utilities|Time|GetWorldDeltaSeconds) 1e+02) 0.0) false false))

(event Input|AxisEvents|InputAxisTurnRight
  (params (AxisValue :type Float%20%28single-precision%29))
  ;[0.6359 0.1323 1] Tank Movement
  (Class|TankMovementComponent|IntendTurnRight (Variables|Default|GetTankMovement) AxisValue))

(event Input|AxisEvents|InputAxisMoveForward
  (params (AxisValue :type Float%20%28single-precision%29))
  ;[0.6359 0.1323 1] Tank Movement
  (Class|TankMovementComponent|IntendMoveForward (Variables|Default|GetTankMovement) AxisValue))

(fn ConstructionScript)